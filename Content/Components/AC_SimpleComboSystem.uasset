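; Actor component that runs a simple attack combo, stepping through an array of animations on successive attacks.
; Attack asks the owner to disable movement, broadcasts the current animation, advances the index and sets a reset timer.
; ComboReset zeroes the index and re-enables owner movement, also running when no valid animation remains.
; SelectAnimation is a bounds-checked lookup that Attack does not use, and ResetOwnerMovement is empty.
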(event Custom|ComboReset
  (Variables|Default|SetAttackIndex 0)
  (Class|BPItoPlayer|EnableMovement(Message) (Components|GetOwner)))

(event Custom|Attack
  (bind _attackindex (Variables|Default|GetAttackIndex))
  (bind _attacksarray (Variables|Default|GetAttacksArray))
  (bind _output (Utilities|Array|Get(acopy) _attacksarray _attackindex))
  ;[0.15 0.15 0.15 0.5] If the owner can move, blocks it
  (bind _result (Class|BPItoPlayer|DisableMovement(Message) (Components|GetOwner)))
  (if _result
    ;[0.15 0.15 0.15 0.5] Selects attack animation and increments "Attack Index"
    (Utilities|IsValid _output
      (:Is%20Valid
        (Default|CallAnimationChanged _output)
        (Math|Integer|IncrementInt (Variables|Default|GetAttackIndex)
          (:%20%20
            ;[0.15 0.15 0.15 0.5] Set timer for combo reset
            (Utilities|Time|SetTimerbyEvent (EventDispatchers|CreateEvent :!event Custom|ComboReset) 2.0))))
      (:Is%20Not%20Valid
        ;[0.15 0.15 0.15 0.5] When there are no more new animation to play in AttacksArray, the combo resets
        (CallFunction|ComboReset)))))

(fn SelectAnimation
  (params (Index :type Integer))
  (bind _attacksarray (Variables|Default|GetAttacksArray))
  (if (>= Index (Utilities|Array|Length (Variables|Default|GetAttacksArray)))
    (CallFunction|ComboReset)
    (return (Utilities|Array|Get(acopy) _attacksarray (Utilities|Array|LastIndex _attacksarray)))
    (else
      (return (Utilities|Array|Get(acopy) (Variables|Default|GetAttacksArray) Index)))))

(fn ResetOwnerMovement)