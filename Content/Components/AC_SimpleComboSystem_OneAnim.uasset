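; AC_SimpleComboSystem_OneAnim is a component that drives an attack combo contained in a single anim montage.
; Attack starts playback through CallPlayAnimation, or sets ContinueCombo if the montage is already playing on the given mesh.
; CheckContinueCombo consumes that flag to let the montage continue, otherwise it re-enables movement through CanMove and stops playback through CallStopAnimation.
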(fn Attack
  (params (Mesh :type Skeletal%20Mesh%20Component%20Object%20Reference))
  ;[0.15 0.15 0.15 0.5] If an anim montage is playing, the animation must continue. If not, it start the animation from the beginning
  (if (Animation|Montage|MontageIsPlaying (Components|SkeletalMesh|GetAnimInstance Mesh) (Variables|Default|GetMontage))
    (Variables|Default|SetContinue%20Combo true)
    (else
      (Default|CallPlayAnimation))))

(fn CheckContinueCombo
  ;[0.15 0.15 0.15 0.5] Checks if the animation must stop or not
  (if (Variables|Default|GetContinue%20Combo)
    (Variables|Default|SetContinue%20Combo false)
    (else
      (Variables|Default|SetCan%20Move true)
      (Default|CallStopAnimation))))